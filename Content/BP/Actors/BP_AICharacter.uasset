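; BP_AICharacter is an AI character that roams, chases the player when perception senses them, and shows its current state in a widget.
; Perception updates write the seen player or last seen location to the state machine's data store, fire gameplay-tag transitions, and switch walk speed between roam and chase.
; On state change it updates the debug label and, entering Chase Player, asks the game mode to start an expanding radius effect at its location.
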(event `self.ReceiveBeginPlay`
  (set `CharacterMovementComponent.MaxWalkSpeed` (`self.RoamSpeed`) (`self.CharacterMovement`))
  (`StateMachine.Run` (`self.BP_AIStateMachine`)))

(event `self.AIPerception.OnTargetPerceptionUpdated`
  (params (Actor :type "Actor Object Reference") (Stimulus :type "AIStimulus Structure"))
  (bind _charactermovement (`self.CharacterMovement`))
  (if (`self.ActorHasTag` Actor "Player")
    (if Stimulus_bSuccessfullySensed
      (bind _returnvalue (`StateMachine.GetDataStore` (`self.BP_AIStateMachine`)))
      (message `/Game/BP/Interfaces/BPI_DataStoreHooks.SetSeenPlayer` _returnvalue Actor)
      (`StateMachine.Transition` (`self.BP_AIStateMachine`) (make `GameplayTag` (struct :`TagName` "T.HasSightOfPlayer")))
      (set `CharacterMovementComponent.MaxWalkSpeed` (`self.ChaseSpeed`) _charactermovement)
      (else
        (bind _returnvalue_2 (`StateMachine.GetDataStore` (`self.BP_AIStateMachine`)))
        (message `/Game/BP/Interfaces/BPI_DataStoreHooks.SetLastSeenLocation` _returnvalue_2 Stimulus_StimulusLocation)
        (`StateMachine.Transition` (`self.BP_AIStateMachine`) (make `GameplayTag` (struct :`TagName` "T.LostSightOfPlayer")))
        (set `CharacterMovementComponent.MaxWalkSpeed` (`self.RoamSpeed`) _charactermovement)))))

(event `self.BP_AIStateMachine.OnChangedStates`
  (params (PreviousState :type "GameplayTag Structure") (CurrentState :type "GameplayTag Structure"))
  (bind _aswbp_log_state_changes (cast `/Game/BP/Widget/WBP_LogStateChanges` (`WidgetComponent.GetUserWidgetObject` (`self.Widget`))))
  (`TextBlock.SetText` (`/Game/BP/Widget/WBP_LogStateChanges.Txt_CurrentState` _aswbp_log_state_changes) (`KismetTextLibrary.Conv_StringToText` (`BlueprintGameplayTagLibrary.GetDebugStringFromGameplayTag` CurrentState)))
  (`|SwitchGameplayTag` CurrentState
    (:`States.ChasePlayer`
      (message `/Game/BP/Interfaces/BPI_Effect.StartEffect` (`GameplayStatics.GetGameMode`) 2.0 100.0 10000.0 (`self.K2_GetActorLocation`)))))

(event `Stop Effect`)

(fn `UserConstructionScript`)