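; BP_Roam is an AI state that makes its owning actor wander between random nearby points while active.
; On entry it requests a random location around the actor from its outer object, falling back to the current position, and issues an AI MoveTo.
; When the move finishes or fails, a delayed timer repeats the cycle if still active.
; Exit invalidates the timer handle and stops movement.
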(event `self.OnEntry`
  (params (GeneralData :type "DataStoreBase Object Reference"))
  (`self.MoveTo`))

(event `MoveTo`
  (bind _returnvalue (`self.GetOwnerActor`))
  (bind _returnvalue_2 (`self.GetOwnerActor`))
  (bind _returnvalue_3 (`Actor.K2_GetActorLocation` _returnvalue))
  (if (and (`KismetSystemLibrary.IsValid` _returnvalue_2) (`KismetSystemLibrary.IsValid` (`AIBlueprintHelperLibrary.GetAIController` _returnvalue_2)))
    (bind (_wassuccessful _randomlocation) (message `/Game/BP/Interfaces/BPI_RandomLocation.GetRandomLocation` (`KismetSystemLibrary.GetOuterObject` self) _returnvalue_3 1000.0))
    (`AITask_MoveTo.AIMoveTo` (`AIBlueprintHelperLibrary.GetAIController` _returnvalue) (select `bool` _wassuccessful :`false` _returnvalue_3 :`true` _randomlocation) null
      (:`OnRequestFailed`
        _)
      (:`OnMoveFinished`
        _))
    (if (`self.IsActive`)
      (bind _returnvalue_4 (`KismetSystemLibrary.K2_SetTimer` self "MoveTo" (`self.Delay`)))
      (set `self.LoopHandle` _returnvalue_4))))

(event `self.OnExit`
  (params (GeneralData :type "DataStoreBase Object Reference"))
  (bind _returnvalue (`AIBlueprintHelperLibrary.GetAIController` (`self.GetOwnerActor`)))
  (`KismetSystemLibrary.K2_InvalidateTimerHandle` (`self.LoopHandle`))
  (`/Engine/EditorBlueprintResources/StandardMacros.IsValid` _returnvalue
    (:`Is Valid`
      (`Controller.StopMovement` _returnvalue))))