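; AI state machine state that sends the agent to the player's last seen location, read from the data passed in on entry.
; When the move finishes or fails while the state is still active, a two-second timer fires the transition toward Roam.
; On exit, such as when perception spots the player, it invalidates that timer and stops movement, so a stale move callback cannot trigger an unwanted transition.
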(event `self.OnEntry`
  (params (GeneralData :type "DataStoreBase Object Reference"))
  (bind _returnvalue (`AIBlueprintHelperLibrary.GetAIController` (`self.GetOwnerActor`)))
  (if (and (`KismetSystemLibrary.DoesImplementInterface` GeneralData "/Game/BP/Interfaces/BPI_DataStoreHooks.BPI_DataStoreHooks_C") (`KismetSystemLibrary.IsValid` _returnvalue))
    (bind _lastseenlocation (message `/Game/BP/Interfaces/BPI_DataStoreHooks.GetLastSeenLocation` GeneralData))
    (`AITask_MoveTo.AIMoveTo` _returnvalue _lastseenlocation null
      (:`OnRequestFailed`
        _)
      (:`OnMoveFinished`
        _))
    ;[1 1 1] Why this? we might be going to the last seen location and we see the player.  so either we transition to chase player, this function call us back with move complete(fail or success), at this point we'll be inadvertly calling next state which is not necessary. So only call next state if needed
    (if (`self.IsActive`)
      ;[1 1 1] Wait before going back to 'Roam'
      (bind _returnvalue_2 (`KismetSystemLibrary.K2_SetTimerDelegate` (delegate `Go to Roam`) 2.0))
      (set `self.DelayHandle` _returnvalue_2))))

(event `Go to Roam`
  (`StateMachine.Transition` (`self.GetStateMachine`) (make `GameplayTag` (struct :`TagName` "T.ArrivedLastSeenLocation"))))

(event `self.OnExit`
  (params (GeneralData :type "DataStoreBase Object Reference"))
  ;[1 1 1] If explicitly told to exit (by the perception component because we've seen the player) but we were waiting to transition to roam state, invalidate handle
  (`KismetSystemLibrary.K2_InvalidateTimerHandle` (`self.DelayHandle`))
  (`Controller.StopMovement` (`AIBlueprintHelperLibrary.GetAIController` (`self.GetOwnerActor`))))