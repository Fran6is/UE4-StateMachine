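; BP_ChasePlayer is an AI state that chases the seen player.
; On entry it stores the general data object and reads the target from it through BPI_DataStoreHooks to drive AIMoveTo.
; When a move finishes or fails, a two-second timer repeats the chase while the state is active.
; Exit stops movement and invalidates the timer handle variable, without explicitly clearing the timer.
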(event `self.OnEntry`
  (params (GeneralData :type "DataStoreBase Object Reference"))
  (set `self.Store` GeneralData)
  (`self.MoveToPlayer`))

(event `MoveToPlayer`
  (bind _returnvalue (`AIBlueprintHelperLibrary.GetAIController` (`self.GetOwnerActor`)))
  (if (and (`KismetSystemLibrary.DoesImplementInterface` (`self.Store`) "/Game/BP/Interfaces/BPI_DataStoreHooks.BPI_DataStoreHooks_C") (`KismetSystemLibrary.IsValid` _returnvalue))
    (bind _seenactor (message `/Game/BP/Interfaces/BPI_DataStoreHooks.GetSeenPlayer` (`self.Store`)))
    (`AITask_MoveTo.AIMoveTo` _returnvalue (0.0 0.0 0.0) _seenactor 100.0
      (:`OnRequestFailed`
        _)
      (:`OnMoveFinished`
        _))
    (if (`self.IsActive`)
      (bind _returnvalue_2 (`KismetSystemLibrary.K2_SetTimer` self "MoveToPlayer" 2.0))
      (set `self.LoopHandle` _returnvalue_2))))

(event `self.OnExit`
  (params (GeneralData :type "DataStoreBase Object Reference"))
  (bind _returnvalue (`AIBlueprintHelperLibrary.GetAIController` (`self.GetOwnerActor`)))
  (`KismetSystemLibrary.K2_InvalidateTimerHandle` (`self.LoopHandle`))
  (`/Engine/EditorBlueprintResources/StandardMacros.IsValid` _returnvalue
    (:`Is Valid`
      (`Controller.StopMovement` _returnvalue))))